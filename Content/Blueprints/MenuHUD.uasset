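; MenuHUD is the main menu HUD for Race Mazer, showing the game title with Play and Quit buttons.
; DrawHUD calls DrawMenu, which draws each button as a textured rectangle with a label and a named hit box at fixed screen coordinates.
; HitBoxClick stores the clicked box name, and GetMenuAction uses it to either open the Maze_0001 level or quit.
; The nodes that store screen width and height are unconnected and never run.
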(event EventDrawHUD
  (params (SizeX :type Integer) (SizeY :type Integer))
  ;[1 1 1] Draw menu on the HUD
  (CallFunction|DrawMenu))

(event EventHitBoxClick
  (params (BoxName :type Name))
  ;[1 1 1] When hit box is clicked
  (Variables|Default|SetHitBoxAction BoxName)
  (CallFunction|GetMenuAction))

(fn ConstructionScript)

(fn DrawMenu
  ;[1 1 1] Print Game Title
  (HUD|DrawText "RACE MAZER" "(R=1.000000,G=1.000000,B=1.000000,A=1.000000)" 1e+02 1e+02 0 1.0 false)
  ;[1 1 1] Draw Play menu text and buttons
  (Class|HUD|AddHitBox "(X=150.000000,Y=150.000000)" "(X=200.000000,Y=50.000000)" "Play" false)
  (Canvas|DrawTexture "/Game/Assets/Textures/T_FloorMarble_D.T_FloorMarble_D" 1.5e+02 1.5e+02 2e+02 5e+01 0.0 0.0 0.0 0.0 "(R=1.000000,G=1.000000,B=1.000000,A=1.000000)")
  (HUD|DrawText "Play" "(R=0.000000,G=0.000000,B=0.000000,A=1.000000)" 1.7e+02 1.7e+02 0 1.0 false)
  ;[1 1 1] Draw Quit menu text and buttons
  (Class|HUD|AddHitBox "(X=150.000000,Y=250.000000)" "(X=200.000000,Y=50.000000)" "Quit" false)
  (Canvas|DrawTexture "/Game/Assets/Textures/T_FloorMarble_D.T_FloorMarble_D" 1.5e+02 2.5e+02 2e+02 5e+01 0.0 0.0 0.0 0.0 "(R=1.000000,G=1.000000,B=1.000000,A=1.000000)")
  (HUD|DrawText "Quit" "(R=0.000000,G=0.000000,B=0.000000,A=1.000000)" 1.7e+02 2.7e+02 0 1.0 false))

(fn GetMenuAction
  (switch string (Utilities|String|ToString(Name) (Variables|Default|GetHitBoxAction))
    (:Play
      ;[1 1 1] If HitBox == Play
      (CallFunction|PlayLevel))
    (:Quit
      ;[1 1 1] If HitBox == Quit
      (CallFunction|ExitGame))))

(fn PlayLevel
  (Development|PrintString "Loading...")
  (Game|OpenLevel(byName) "Maze_0001"))

(fn ExitGame
  (Game|QuitGame))