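; TimerHUD is a HUD Blueprint whose GetCurrentGameTime function draws the elapsed game time in white at a fixed screen position.
; FormatTime joins minutes, seconds and a "jiffy" field with colons, using AddLeadingZero to pad each to two digits.
; The jiffy field takes time times 100 modulo 60, so it wraps at 60 rather than showing true hundredths.
; No event in the file calls the draw function.
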(fn ConstructionScript)

(fn FomatJiffy
  (params (CurrentGameTime :type Float%20%28single-precision%29))
  (bind _formattedstring (CallFunction|AddLeadingZero (Math|Float|Floor (.Remainder (Math|Float|Division(WholeandRemainder) (* CurrentGameTime 1e+02) 6e+01)))))
  (return _formattedstring))

(fn FormatSeconds
  (params (CurrentGameTime :type Float%20%28single-precision%29))
  (bind _formattedstring (CallFunction|AddLeadingZero (Math|Float|Floor (.Remainder (Math|Float|Division(WholeandRemainder) CurrentGameTime 6e+01)))))
  (return _formattedstring))

(fn FormatMinutes
  (params (CurrentGameTime :type Float%20%28single-precision%29))
  (bind _formattedstring (CallFunction|AddLeadingZero (.ReturnValue (Math|Float|Division(WholeandRemainder) CurrentGameTime 6e+01))))
  (return _formattedstring))

(fn GetCurrentGameTime
  (bind _formattedgametime (CallFunction|FormatTime (Utilities|Time|GetGameTimeinSeconds)))
  (HUD|DrawText _formattedgametime "(R=1.000000,G=1.000000,B=1.000000,A=1.000000)" 5e+02 4e+01 0 1.0 false))

(fn FormatTime
  (params (CurrentGameTime :type Float%20%28single-precision%29))
  (bind _minutes (CallFunction|FormatMinutes CurrentGameTime))
  (bind _seconds (CallFunction|FormatSeconds CurrentGameTime))
  (bind _jiffy (CallFunction|FomatJiffy CurrentGameTime))
  (return (Utilities|String|Append (Utilities|String|Append _minutes ":") (Utilities|String|Append (Utilities|String|Append _seconds ":") _jiffy))))

(fn AddLeadingZero
  (params (IntToFormat :type Integer))
  (Variables|Default|SetFormattedString (Utilities|String|ToString(Integer) IntToFormat))
  (if (< IntToFormat 10)
    (Variables|Default|SetFormattedString (Utilities|String|Append "0" (Variables|Default|GetFormattedString))))
  (return (Variables|Default|GetFormattedString)))