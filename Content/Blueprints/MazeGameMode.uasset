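; MazeGameMode is a Blueprint for a maze game that sets up the game phase on play start.
; BeginPlay switches on GamePart to call a handler for the begin, main, end or menu phase.
; All four handlers, including the main game's, set global time dilation to zero.
; The pause and unpause calls in the begin, main and end handlers are unconnected and never run.
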(event EventBeginPlay
  (switch string (Variables|Default|GetGamePart)
    (:BeginGame
      (CallFunction|BeginGamePart))
    (:MainGame
      (CallFunction|MainGamePart))
    (:EndGame
      (CallFunction|EndGamePart))
    (:Menu
      (CallFunction|MenuPart))))

(fn ConstructionScript)

(fn BeginGamePart
  (Utilities|Time|SetGlobalTimeDilation 0.0))

(fn MainGamePart
  (Utilities|Time|SetGlobalTimeDilation 0.0))

(fn EndGamePart
  (Utilities|Time|SetGlobalTimeDilation 0.0))

(fn MenuPart
  (Utilities|Time|SetGlobalTimeDilation 0.0))