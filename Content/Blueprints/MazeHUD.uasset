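; MazeHUD is the maze game's canvas HUD, drawing a different screen for each game phase.
; DrawHUD switches on the game mode's GamePart: a delayed 3-2-1 countdown leading into main game, a main screen, or placeholder End Game and Menu text.
; The main screen shows a Menu label and game time formatted by zero-padding helpers.
; A Pause hit-box click toggles pause, but DisplayPause, which creates that box, is never called.
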(event EventHitBoxClick
  (params (BoxName :type Name))
  ;[1 1 1] Pause
  (switch string (Utilities|String|ToString(Name) BoxName)
    (:Pause
      (CallFunction|PauseGame))))

(event EventDrawHUD
  (params (SizeX :type Integer) (SizeY :type Integer))
  (switch string (Variables|/Game/Blueprints/MazeGameMode.MazeGameMode_C|GetGamePart (Variables|Default|GetMazeGameMode))
    (:BeginGame
      ;[1 1 1] Begin Game (Start Countdown)
      (Development|PrintString "3")
      (HUD|DrawText "3" "(R=0.000000,G=0.000000,B=0.000000,A=1.000000)" 2e+02 2e+02 0 5.0 false)
      (Utilities|FlowControl|Delay 1.0)
      (Development|PrintString "2")
      (HUD|DrawText "2" "(R=0.000000,G=0.000000,B=0.000000,A=1.000000)" 2e+02 2e+02 0 5.0 false)
      (Utilities|FlowControl|Delay 1.0)
      (Development|PrintString "1")
      (HUD|DrawText "1" "(R=0.000000,G=0.000000,B=0.000000,A=1.000000)" 2e+02 2e+02 0 5.0 false)
      (Utilities|FlowControl|Delay 5.0)
      (Development|PrintString "Begin")
      (Variables|/Game/Blueprints/MazeGameMode.MazeGameMode_C|SetGamePart (Variables|Default|GetMazeGameMode) "MainGame"))
    (:MainGame
      ;[1 1 1] Draw Heads-up Display (HUD) for Main Game
      (CallFunction|DrawMainGameHUD))
    (:EndGame
      ;[1 1 1] End Game
      (CallFunction|EndGameHUD))
    (:Menu
      ;[1 1 1] Menu
      (CallFunction|MenuHUD))))

(event EventBeginPlay
  ;[1 1 1] Calls Game Begin
  (if (Utilities|Text|TextIsEmpty (Utilities|Text|ToText(String) (Variables|/Game/Blueprints/MazeGameMode.MazeGameMode_C|GetGamePart (Variables|Default|GetMazeGameMode))))
    (Variables|/Game/Blueprints/MazeGameMode.MazeGameMode_C|SetGamePart (Variables|Default|GetMazeGameMode) "BeginGame")))

(fn ConstructionScript)

(fn DisplayTimer
  ;[1 1 1] Display Timer
  (bind _newparam (CallFunction|FormatTime (Utilities|Time|GetGameTimeinSeconds)))
  (HUD|DrawText _newparam "(R=0.195533,G=0.705743,B=0.920000,A=1.000000)" 3e+02 1e+01 0 2.0 false))

(fn DisplayPause
  (HUD|DrawText "Pause" "(R=1.000000,G=1.000000,B=1.000000,A=1.000000)" 5e+02 6e+02 0 1.0 false)
  (Class|HUD|AddHitBox "(X=500.000000,Y=600.000000)" "(X=100.000000,Y=100.000000)" "Pause" false))

(fn PauseGame
  (Variables|Default|SetisPaused (not (Variables|Default|GetisPaused)))
  (Game|SetGamePaused (not (Variables|Default|GetisPaused))))

(fn FormatTime
  (params (TimeToFormat :type Float%20%28single-precision%29))
  (bind _minutes (CallFunction|GetMinutes TimeToFormat))
  (bind _seconds (CallFunction|GetSeconds TimeToFormat))
  (bind _jiffy (CallFunction|GetJiffy TimeToFormat))
  (return (Utilities|String|Append (Utilities|String|Append (Utilities|String|Append _minutes ":") (Utilities|String|Append _seconds ":")) (Utilities|String|Append "" _jiffy))))

(fn GetSeconds
  (params (TimetoFormat :type Float%20%28single-precision%29))
  (bind _formattedtime (CallFunction|AddLeadingZero (Math|Float|Floor (Math|Float|%(Float) TimetoFormat 6e+01))))
  (return _formattedtime))

(fn GetJiffy
  (params (TimeToFormat :type Float%20%28single-precision%29))
  (bind _formattedtime (CallFunction|AddLeadingZero (Math|Float|Floor (Math|Float|%(Float) (* TimeToFormat 1e+03) 6e+01))))
  (return _formattedtime))

(fn GetMinutes
  (params (TimeToFormat :type Float%20%28single-precision%29))
  (bind _formattedtime (CallFunction|AddLeadingZero (.ReturnValue (Math|Float|Division(WholeandRemainder) TimeToFormat 6e+01))))
  (return _formattedtime))

(fn AddLeadingZero
  (params (TimeToFormat :type Integer))
  (Variables|Default|SetFormattedTime (Utilities|String|ToString(Integer) TimeToFormat))
  (if (< TimeToFormat 10)
    (Variables|Default|SetFormattedTime (Utilities|String|Append "0" (Variables|Default|GetFormattedTime))))
  (return (Variables|Default|GetFormattedTime)))

(fn DrawMainGameHUD
  (Canvas|DrawTexture "/Game/Assets/Textures/T_Crackle.T_Crackle" 5e+01 2e+01 1e+02 5e+01 0.0 0.0 0.0 0.0 "(R=1.000000,G=1.000000,B=1.000000,A=1.000000)")
  (HUD|DrawText "Menu" "(R=1.000000,G=1.000000,B=1.000000,A=1.000000)" 5e+01 2e+01 0 1.0 false)
  (CallFunction|DisplayTimer))

(fn EndGameHUD
  (HUD|DrawText "End Game" "(R=1.000000,G=1.000000,B=1.000000,A=1.000000)" 0.0 0.0 0 1.0 false))

(fn MenuHUD
  (HUD|DrawText "Menu" "(R=1.000000,G=1.000000,B=1.000000,A=1.000000)" 0.0 0.0 0 1.0 false))