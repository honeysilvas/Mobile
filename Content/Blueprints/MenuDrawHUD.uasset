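; HUD Blueprint that draws the RACE MAZER menu, with a title and Play and Quit buttons.
; DrawHUD paints it directly each frame, layering a named hit box, a marble texture and a text label for each button.
; Layout uses fixed pixel positions, as the screen width and height assignments are not connected.
; No hit box click handling is defined here.
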(event EventDrawHUD
  (params (SizeX :type Integer) (SizeY :type Integer))
  ;[1 1 1] Print Game Title
  (HUD|DrawText "RACE MAZER" "(R=1.000000,G=1.000000,B=1.000000,A=1.000000)" 1e+02 1e+02 0 1.0 false)
  ;[1 1 1] Draw Play menu text and buttons
  (Class|HUD|AddHitBox "(X=150.000000,Y=150.000000)" "(X=200.000000,Y=50.000000)" "Play" false)
  (Canvas|DrawTexture "/Game/Assets/Textures/T_FloorMarble_D.T_FloorMarble_D" 1.5e+02 1.5e+02 2e+02 5e+01 0.0 0.0 0.0 0.0 "(R=1.000000,G=1.000000,B=1.000000,A=1.000000)")
  (HUD|DrawText "Play" "(R=0.000000,G=0.000000,B=0.000000,A=1.000000)" 1.7e+02 1.7e+02 0 1.0 false)
  ;[1 1 1] Draw Quit menu text and buttons
  (Class|HUD|AddHitBox "(X=150.000000,Y=250.000000)" "(X=200.000000,Y=50.000000)" "Quit" false)
  (Canvas|DrawTexture "/Game/Assets/Textures/T_FloorMarble_D.T_FloorMarble_D" 1.5e+02 2.5e+02 2e+02 5e+01 0.0 0.0 0.0 0.0 "(R=1.000000,G=1.000000,B=1.000000,A=1.000000)")
  (HUD|DrawText "Quit" "(R=0.000000,G=0.000000,B=0.000000,A=1.000000)" 1.7e+02 2.7e+02 0 1.0 false))

(fn ConstructionScript)